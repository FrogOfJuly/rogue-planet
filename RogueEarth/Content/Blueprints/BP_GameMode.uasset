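; Game mode Blueprint that mirrors a thermal simulation from BP_SolverManager into scene materials and tracks temperature and days passed.
; A delay-gated Tick periodically reads the solver's temperature and iteration, storing a Celsius readout.
; Land uses the solver temperature directly, while water, leaves and trunk step down from it by heat coefficients relative to ground.
; Each temperature is normalized with a fixed offset and written to the MPC_Thermal parameter collection.
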(event `UpdateMaterials`
  (`|ExecutionSequence`
    (:`then_0`
      (bind _alpha (`self.GetNewAlpha` (`self.CurT`)))
      (`KismetMaterialLibrary.SetScalarParameterValue` "/Game/Materials/MPC_Thermal.MPC_Thermal" "LandCoef" _alpha))
    (:`then_1`
      (bind _newt (`self.GetObjectTemp` (`self.CurWaterT`) (`.TempCoef` (break `HeatCapacity` (`HeatConfig.Water` (`self.HeatConfig`))))))
      (bind _output_get (set `self.CurWaterT` _newt))
      (bind _alpha_2 (`self.GetNewAlpha` _output_get))
      (`KismetMaterialLibrary.SetScalarParameterValue` "/Game/Materials/MPC_Thermal.MPC_Thermal" "WaterCoef" _alpha_2))
    (:`then_2`
      (bind _newt_2 (`self.GetObjectTemp` (`self.CurLeavesT`) (`.TempCoef` (break `HeatCapacity` (`HeatConfig.Leaves` (`self.HeatConfig`))))))
      (bind _output_get_2 (set `self.CurLeavesT` _newt_2))
      (bind _alpha_3 (`self.GetNewAlpha` _output_get_2))
      (`KismetMaterialLibrary.SetScalarParameterValue` "/Game/Materials/MPC_Thermal.MPC_Thermal" "LeavesCoef" _alpha_3))
    (:`then_3`
      (bind _newt_3 (`self.GetObjectTemp` (`self.CurTrunkT`) (`.TempCoef` (break `HeatCapacity` (`HeatConfig.Trunk` (`self.HeatConfig`))))))
      (bind _output_get_3 (set `self.CurTrunkT` _newt_3))
      (bind _alpha_4 (`self.GetNewAlpha` _output_get_3))
      (`KismetMaterialLibrary.SetScalarParameterValue` "/Game/Materials/MPC_Thermal.MPC_Thermal" "TrunkCoef" _alpha_4))))

(event `self.ReceiveBeginPlay`
  (bind _maxt (`self.MaxT`))
  (bind _returnvalue (`GameplayStatics.GetActorOfClass` "/Game/BP_SolverManager.BP_SolverManager_C"))
  (bind _output_get (set `self.Solver` _returnvalue))
  (set `self.StepDelay` (`self.InitStepDelay`))
  (bind _returnvalue_2 (`SolverManager.GetIterations` _output_get))
  (set `self.AllDays` _returnvalue_2)
  (set `self.CurT` _maxt)
  (set `self.CurWaterT` _maxt)
  (set `self.CurLeavesT` _maxt)
  (set `self.CurTrunkT` _maxt))

(event `IterStep`
  (bind _solver (`self.Solver`))
  (`|ExecutionSequence`
    (:`then_0`
      (bind _returnvalue (`SolverManager.getT` _solver))
      (bind _output_get (set `self.CurT` _returnvalue))
      (set `self.CurrentT` (`KismetMathLibrary.FTrunc` (`self.KtoC` _output_get)))
      (`self.UpdateMaterials`))
    (:`then_1`
      (bind _returnvalue_2 (`SolverManager.GetCurrentIteration` _solver))
      (set `self.DaysPassed` _returnvalue_2))))

(event `self.ReceiveTick`
  (params (DeltaSeconds :type "Float (single-precision)"))
  (if (not (`self.IsInIter`))
    (set `self.IsInIter` true)
    (`self.IterStep`)
    (`KismetSystemLibrary.Delay` (`self.StepDelay`))
    (set `self.IsInIter` false)))

(fn `GetNewAlpha`
  (params (newT :type "Float (double-precision) (by ref)"))
  (returns (alpha :type "Float (double-precision)"))
  (return (- (/ (- newT (`self.MinT`)) (- (`self.MaxT`) (`self.MinT`))) 0.23)))

(fn `GetObjectTemp`
  (params (OldT :type "Float (double-precision)") (HeatCoef :type "Float (double-precision)"))
  (returns (NewT :type "Float (double-precision)"))
  (return (- OldT (/ (`KismetMathLibrary.Abs` (- OldT (`self.CurT`))) (/ HeatCoef (`.TempCoef` (break `HeatCapacity` (`HeatConfig.Ground` (`self.HeatConfig`)))))))))

(fn `KtoC`
  (params (TK :type "Float (double-precision)"))
  (returns (TC :type "Float (double-precision)"))
  (return (- TK 273.149994)))

(fn `UserConstructionScript`)